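; Enemy AI pawn that chases the player once spotted and plays a montage on reaching them.
; PawnSensing sets a seeing flag and calls FollowPlayer, which casts the player to BP_ThirdPersonCharacter and issues AIMoveTo toward it.
; On arrival, a CanAttack flag and montage-length delay gate the montage, though each FollowPlayer call re-enables the flag.
; Tick halts movement while the flag is false; once set by sighting, it is effectively never cleared.
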(event OnSeePawn(PawnSensing)
  (params (Pawn :type Pawn%20Object%20Reference))
  (Variables|Default|SetisSeeingPlayer? true)
  (CallFunction|FollowPlayer))

(event Custom|FollowPlayer
  (Utilities|FlowControl|Sequence
    (:then_0
      (Variables|Default|SetcanAttack? true)
      (if (Variables|Default|GetisSeeingPlayer?)
        (AI|AIMoveTo self "0, 0, 0" (stale _asbp_third_person_character) 7e+01 false :!label _label
          (:OnSuccess
            (if (Variables|Default|GetcanAttack?)
              (Variables|Default|SetcanAttack? false)
              (bind _returnvalue (Animation|PlayAnimMontage 0 1.0 "None"))
              (Utilities|FlowControl|Delay _returnvalue)
              (Variables|Default|SetcanAttack? true))))
        (else
          (Variables|Default|SetisSeeingPlayer? false))))
    (:then_1
      (bind _asbp_third_person_character (Utilities|Casting|CastToBP_ThirdPersonCharacter (Game|GetPlayerCharacter 0)))
      (goto _label))))

(event EventBeginPlay)

(event EventTick
  (params (DeltaSeconds :type Float%20%28single-precision%29))
  (if (not (Variables|Default|GetisSeeingPlayer?))
    (Components|Movement|StopMovementImmediately (Variables|Character|GetCharacterMovement))))

(fn ConstructionScript)